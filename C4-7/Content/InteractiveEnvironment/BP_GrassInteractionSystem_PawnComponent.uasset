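; Pawn component that feeds grass interaction materials a six-slot trail of virtual particles through MC_GrassInteractionSimple.
; Tick tracks the owner's foot location and derives velocity from movement deltas, so no movement component is required.
; A looping timer overwrites slots round-robin with location, velocity and spawn time in alpha.
; BeginPlay sets trail radius, falloff and timescale to match slot reuse, and optionally starts debug drawing.
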(event `self.ReceiveBeginPlay`
  (bind _returnvalue (`self.GetOwner`))
  ;[1 1 1] cache owner's location right away & reset velocity
  (`/Engine/EditorBlueprintResources/StandardMacros.IsValid` _returnvalue
    (:`Is Valid`
      (set `self.PawnLocation` (`Actor.K2_GetActorLocation` _returnvalue))
      (set `self.PawnVelocity` (0.0 0.0 0.0))
      ;[1 1 1] tell material the radius of each particle
      (`KismetMaterialLibrary.SetScalarParameterValue` "/Game/InteractiveEnvironment/Foliage/InteractiveGrassElements/Collections/MC_GrassInteractionSimple.MC_GrassInteractionSimple" "TrailRadius" (`self.ParticleRadius`))
      (`KismetMaterialLibrary.SetScalarParameterValue` "/Game/InteractiveEnvironment/Foliage/InteractiveGrassElements/Collections/MC_GrassInteractionSimple.MC_GrassInteractionSimple" "TrailRadiusFalloff" (`self.ParticleRadiusFalloff`))
      ;[1 1 1] tell material how much time each particle can 'live' before being spawned again. Each particle should reach its end of life right at the time it's spawn again and so for 6 particles, it's 1/(spawnrate * 6)
      (`KismetMaterialLibrary.SetScalarParameterValue` "/Game/InteractiveEnvironment/Foliage/InteractiveGrassElements/Collections/MC_GrassInteractionSimple.MC_GrassInteractionSimple" "TrailTimescale" (/ 1.0 (* (`self.ParticleSpawnRate`) 6.0)))
      ;[1 1 1] start timer to spawn virtual particles at a constant interval
      (`KismetSystemLibrary.K2_SetTimer` null "IncrementTrailParticles" (`self.ParticleSpawnRate`) true)
      ;[1 1 1] possibly start timer to draw debug info
      (if (`self.bDrawDebug`)
        (`KismetSystemLibrary.K2_SetTimer` null "DrawDebugTrailParticles" (`self.ParticleSpawnRate`) true)))))

(event `self.ReceiveTick`
  (params (DeltaSeconds :type "Float (single-precision)"))
  ;[1 1 1] tick to compute our own velocity and update material
  (`self.UpdateTrailParticles` DeltaSeconds))

(fn `DrawDebugTrailParticles`
  (locals (ThisString :type String) (ThisLocation :type "Vector Structure"))
  (bind _thislocation (`local.ThisLocation`))
  (bind _thislocation_2 (`local.ThisLocation`))
  (bind _particlespawnrate (`self.ParticleSpawnRate`))
  (bind _returnvalue (* (`self.ParticleSpawnRate`) 6.0))
  ;[1 1 1] for each particle
  (for _index (range 6)
    ;[1 1 1] get its location
    (bind _output_get (set `local.ThisString` (`KismetStringLibrary.Concat_StrStr` "Trail" (`KismetStringLibrary.Conv_IntToString` (+ _index 1)))))
    (bind _returnvalue_2 (`KismetMaterialLibrary.GetVectorParameterValue` "/Game/InteractiveEnvironment/Foliage/InteractiveGrassElements/Collections/MC_GrassInteractionSimple.MC_GrassInteractionSimple" (`KismetStringLibrary.Conv_StringToName` (`KismetStringLibrary.Concat_StrStr` _output_get "Location"))))
    (bind (_r _g _b _a) (`KismetMathLibrary.BreakColor` _returnvalue_2))
    (bind _output_get_2 (set `local.ThisLocation` (`KismetMathLibrary.MakeVector` _r _g (+ _b 5.0))))
    ;[1 1 1] draw circle at location
    (`KismetSystemLibrary.DrawDebugCircle` _output_get_2 (`self.ParticleRadius`) 48 (struct :`R` 1.0 :`G` 1.0 :`B` 1.0 :`A` 1.0) (`self.ParticleSpawnRate`) 4.0 (0.0 1.0 0.0) (1.0 0.0 0.0))
    ;[1 1 1] get its velocity
    (bind _returnvalue_3 (`KismetMaterialLibrary.GetVectorParameterValue` "/Game/InteractiveEnvironment/Foliage/InteractiveGrassElements/Collections/MC_GrassInteractionSimple.MC_GrassInteractionSimple" (`KismetStringLibrary.Conv_StringToName` (`KismetStringLibrary.Concat_StrStr` (`local.ThisString`) "Velocity"))))
    (bind (_r_2 _g_2 _b_2) (`KismetMathLibrary.BreakColor` _returnvalue_3))
    ;[1 1 1] draw a debug line for its velocity and one for its alpha
    (`KismetSystemLibrary.DrawDebugLine` _thislocation (+ _thislocation (`KismetMathLibrary.MakeVector` _r_2 _g_2 _b_2)) (struct :`R` 1.0 :`B` 0.1 :`A` 1.0) _particlespawnrate 4.0)
    (`KismetSystemLibrary.DrawDebugLine` _thislocation_2 (+ _thislocation_2 (`KismetMathLibrary.MakeVector` 0.0 0.0 (* (- _returnvalue (`KismetMathLibrary.FClamp` (- (`KismetSystemLibrary.GetGameTimeInSeconds`) _a) 0.0 _returnvalue)) 100.0))) (struct :`R` 1.0 :`G` 1.0 :`B` 1.0 :`A` 1.0) _particlespawnrate 4.0))
  (return))

(fn `IncrementTrailParticles`
  (locals (ThisOwner :type "Actor Object Reference") (ThisLocation :type "Vector Structure") (ParticlelUpdateRate :type "Float (double-precision)") (ThisVelocity :type "Vector Structure") (ThisIndex :type Byte) (ThisAge :type "Float (double-precision)") (ThisString :type String) (ThisName :type Name) (ThisDeltaTime :type "Float (double-precision)" :default 0.0))
  (bind _thisstring (`local.ThisString`))
  ;[1 1 1] loop through the six available particles
  (set `self.ParticleIndex` (mod (+ (`self.ParticleIndex`) 1) 6))
  ;[1 1 1] get step parameter base name
  (set `local.ThisString` (`KismetStringLibrary.Concat_StrStr` "Trail" (`KismetStringLibrary.Conv_IntToString` (+ (`self.ParticleIndex`) 1))))
  ;[1 1 1] store location, time at which this particle is spawned and velocity
  (`KismetMaterialLibrary.SetVectorParameterValue` "/Game/InteractiveEnvironment/Foliage/InteractiveGrassElements/Collections/MC_GrassInteractionSimple.MC_GrassInteractionSimple" (`KismetStringLibrary.Conv_StringToName` (`KismetStringLibrary.Concat_StrStr` _thisstring "Location")) (make `LinearColor` (.x (`self.PawnLocation`)) (.y (`self.PawnLocation`)) (.z (`self.PawnLocation`)) (`KismetSystemLibrary.GetGameTimeInSeconds`)))
  (`KismetMaterialLibrary.SetVectorParameterValue` "/Game/InteractiveEnvironment/Foliage/InteractiveGrassElements/Collections/MC_GrassInteractionSimple.MC_GrassInteractionSimple" (`KismetStringLibrary.Conv_StringToName` (`KismetStringLibrary.Concat_StrStr` _thisstring "Velocity")) (make `LinearColor` (.x (`self.PawnVelocity`)) (.y (`self.PawnVelocity`)) (.z (`self.PawnVelocity`)) 1.0))
  (return))

(fn `UpdateTrailParticles`
  (params (DeltaTime :type "Float (double-precision)"))
  (locals (ThisOwner :type "Actor Object Reference") (ThisLocation :type "Vector Structure") (ParticlelUpdateRate :type "Float (double-precision)") (ThisIndex :type Byte) (ThisAge :type "Float (double-precision)") (ThisString :type String) (ThisName :type Name) (ThisDeltaTime :type "Float (double-precision)" :default 0.0))
  ;[1 1 1] get our owner's latest location and push it downward by a value that should equal to its half-height so that the actual location is at the actor's 'feet' and not its center
  (bind _output_get (set `local.ThisOwner` (`self.GetOwner`)))
  (set `local.ThisLocation` (- (`Actor.K2_GetActorLocation` _output_get) (`KismetMathLibrary.MakeVector` 0.0 0.0 (`self.PawnHalfHeight`))))
  ;[1 1 1] compute our owner's velocity ourself so that we don't rely on our owner having a movement component of some sort to get an actual velocity
  (set `self.PawnVelocity` (/ (- (`local.ThisLocation`) (`self.PawnLocation`)) DeltaTime))
  (set `self.PawnLocation` (`local.ThisLocation`))
  (return))