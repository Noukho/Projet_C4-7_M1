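; BP_Checkpoint is a level checkpoint actor that activates when any actor overlaps it.
; On BeginPlay it caches the c47GameMode, whose current checkpoint is compared against itself to skip re-activation.
; On a new activation it stores the SpawnPosition component's world transform as the spawn transform, calls ActivateCheckpoint and plays a flame sound at that location.
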(event `self.ReceiveBeginPlay`
  (bind _asc_47game_mode (cast `c47GameMode` (`GameplayStatics.GetGameMode`)))
  (set `self.currentGameMode` _asc_47game_mode))

(event `self.ReceiveActorBeginOverlap`
  (params (OtherActor :type "Actor Object Reference"))
  (if (not (== (`c47GameMode.currentCheckpoint` (`self.currentGameMode`)) self))
    (bind _output_get (set `self.checkpointSpawnTransform` (`SceneComponent.K2_GetComponentToWorld` (`self.SpawnPosition`))))
    (`self.ActivateCheckpoint`)
    (`GameplayStatics.PlaySoundAtLocation` "/Game/Sound/SFX/SOUND_DESIGN_FLAME.SOUND_DESIGN_FLAME" (.location _output_get) (struct) 1.0 1.0 0.0 null null null null)))

(fn `UserConstructionScript`)