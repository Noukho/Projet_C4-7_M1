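; BP_Eye is an actor, apparently an eye on a NightDream tree, that turns to watch the player.
; Each tick it checks that the first player character is valid and computes a look-at rotation from its own location to that character.
; It rotates the whole actor toward that rotation with RInterpTo at a fixed speed, so the gaze follows smoothly with some lag.
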(event `self.ReceiveTick`
  (params (DeltaSeconds :type "Float (single-precision)"))
  (if (`KismetSystemLibrary.IsValid` (`GameplayStatics.GetPlayerCharacter` 0))
    (`self.K2_SetActorRotation` (`KismetMathLibrary.RInterpTo` (`self.K2_GetActorRotation`) (`KismetMathLibrary.FindLookAtRotation` (`self.K2_GetActorLocation`) (`self.K2_GetActorLocation` (`GameplayStatics.GetPlayerCharacter` 0))) (`GameplayStatics.GetWorldDeltaSeconds`) 2.0))))

(fn `UserConstructionScript`)